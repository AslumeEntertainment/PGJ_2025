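; Gameplay Ability for an ultimate that shifts the cleanness of nearby PaintableItem actors around the avatar.
; After committing, it plays a montage-slot animation, and on completion the server sphere-overlaps for items.
; The sign of an effectiveness attribute on the avatar's ability system decides whether each item's maximum cleanness is added or subtracted.
; Debug prints and a debug sphere remain, and completion ends the ability only on authority.
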(event Ability|EventActivateAbility
  (bind _returnvalue (Ability|GetAvatarActorfromActorInfo))
  (bind _returnvalue_2 (Transformation|GetActorLocation _returnvalue))
  (bind _returnvalue_3 (Ability|GetAbilitySystemComponent _returnvalue))
  (bind (_bsuccessfullyfoundattribute _returnvalue_4) (Ability|Attribute|GetFloatAttributefromAbilitySystemComponent _returnvalue_3 "(AttributeName=\"Effectiveness\",Attribute=/Script/Bubbles.BubbleAttributeSet:Effectiveness,AttributeOwner=\"/Script/CoreUObject.Class'/Script/Bubbles.BubbleAttributeSet'\")"))
  (bind _returnvalue_5 (Ability|CommitAbility))
  (if _returnvalue_5
    (|PlayAnimandWaitProxy "None" "/Game/Assets/Models/3DPawn/Animations/bubbleman_v1_Anim_Armature_causing_chaos.bubbleman_v1_Anim_Armature_causing_chaos" "DefaultSlot" 0.25 0.25 1.0 0.0 true 1.0
      (:then
        (Development|PrintString "boom"))
      (:OnCompleted
        (Ability|HasAuthority
          (:True
            (Development|PrintString "Domain Expansion")
            (Rendering|Debug|DrawDebugSphere _returnvalue_2 1e+02 12 "(R=1.000000,G=1.000000,B=1.000000,A=1.000000)" 3.0)
            (bind _outactors (Collision|SphereOverlapActors _returnvalue_2 1e+02 (Variables|Default|GetObject%20Types) "/Script/Bubbles.PaintableItem"))
            (Development|PrintString (Utilities|String|ToString(Integer) (Utilities|Array|Length _outactors)))
            (if _bsuccessfullyfoundattribute
              (for _array_element _outactors
                (bind _aspaintable_item (Utilities|Casting|CastToPaintableItem _array_element))
                (Development|PrintString (Utilities|String|Append "Current: " (Utilities|String|ToString(Integer) (Class|PaintableItem|GetCurrentCleanness _aspaintable_item))))
                (Class|PaintableItem|SetCleanness _aspaintable_item (+ (Class|PaintableItem|GetCurrentCleanness _aspaintable_item) (Math|Float|Truncate (* (Class|PaintableItem|GetMaxCleanness _aspaintable_item) (Math|Float|Sign(Float) _returnvalue_4)))) false))
              (else
                (Development|PrintString "No Effectiveness")))
            (Ability|EndAbility)))))
    (else
      (Ability|EndAbility))))

(event Ability|EventOnEndAbility
  (params (bWasCancelled :type Boolean)))

(event Ability|EventActivateAbilityFromEvent
  (params (EventData :type Gameplay%20Event%20Data%20Structure%20%28by%20ref%29)))