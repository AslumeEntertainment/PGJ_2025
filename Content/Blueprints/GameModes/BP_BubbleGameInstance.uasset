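; BP_BubbleGameInstance is the game instance that handles hosting and joining online sessions through Advanced Sessions.
; Hosting creates a two-connection session tagged with a lobby name and GameID, then opens the Kitchen level as a listen server.
; Non-public sessions are marked by appending a friends-edition suffix to the GameID.
; Joining takes a given search result, and network errors destroy the current session.
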(event Custom|HostSession
  (params (SessionName :type String) (bIsPublic :type Boolean))
  (bind _gameid (Variables|Default|GetGameID))
  (if bIsPublic
    (Variables|Default|SetTemp _gameid)
    (else
      (Variables|Default|SetTemp (Utilities|String|Append _gameid ".PlusFriendsEdition"))))
  (|AdvancedSession (Utilities|Array|MakeArray (Class|AdvancedSessionsLibrary|MakeLiteralSessionPropertyString "LobbyName" SessionName) (Class|AdvancedSessionsLibrary|MakeLiteralSessionPropertyString "GameID" (Variables|Default|GetTemp))) (Game|GetPlayerController 0) 2 0 false true false true true true false false false true false true
    (:OnSuccess
      (Game|OpenLevel(byName) "Kitchen" true "?listen"))))

(event Custom|JoinSession
  (params (Session :type Blueprint%20Session%20Result%20Structure))
  (|JoinSession (Game|GetPlayerController 0) Session))

(event EventHandleNetworkError
  (params (FailureType :type ENetworkFailure%20Enum :default "NetDriverAlreadyExists") (bIsServer :type Boolean))
  (|DestroySession (Game|GetPlayerController 0)))