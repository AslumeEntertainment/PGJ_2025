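; Title-screen game mode that hosts, finds and joins multiplayer sessions through the Advanced Sessions plugin.
; HostSession creates a two-connection session with a fixed lobby name and game ID, then opens the Kitchen level as a listen server.
; FindSessions filters by that game ID, caches the results and broadcasts lobby names via OnSessionsFound, sending an empty list on failure.
; JoinSession joins a cached result by index.
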(event EventFindSessions
  (bind _sessionnames (Variables|Default|GetSessionNames))
  (Utilities|Array|Clear (Variables|Default|GetSessionNames))
  (bind _results (|FindSessionsAdvanced (Game|GetPlayerController 0) 50 false "AllServers" (Utilities|Array|MakeArray (Class|AdvancedSessionsLibrary|MakeLiteralSessionSearchProperty (Class|AdvancedSessionsLibrary|MakeLiteralSessionPropertyString "GameID" "BubbleKaisen") "Equals")) false false false true)
    (:OnSuccess
      (bind _output_get (Variables|Default|SetSessions _results))
      (for _array_element _output_get
        (bind _extrasettings (Class|AdvancedSessionsLibrary|GetExtraSettings _array_element))
        (bind _settingvalue (Class|AdvancedSessionsLibrary|GetSessionPropertyString _extrasettings "LobbyName")
          (:Found
            (Utilities|Array|Add _sessionnames (Utilities|Text|ToText(String) _settingvalue))))))
    (:OnFailure
      _))
  (Default|CallOnSessionsFound _sessionnames))

(event EventHostSession
  (|AdvancedSession (Utilities|Array|MakeArray (Class|AdvancedSessionsLibrary|MakeLiteralSessionPropertyString "LobbyName" "Shibuya") (Class|AdvancedSessionsLibrary|MakeLiteralSessionPropertyString "GameID" "BubbleKaisen")) (Game|GetPlayerController 0) 2 0 false true false true true true false false false true false true
    (:OnSuccess
      (Game|OpenLevel(byName) "Kitchen" true "?listen"))))

(event EventJoinSession
  (params (SessionId :type Integer))
  (|JoinSession (Game|GetPlayerController 0) (Utilities|Array|Get(acopy) (Variables|Default|GetSessions) SessionId)))

(fn ConstructionScript)